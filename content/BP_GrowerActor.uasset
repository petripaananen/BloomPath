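; BP_GrowerActor is a plant actor that mirrors Jira task state, with leaves as tagged static mesh components.
; GrowLeaves adds a scaled mesh tagged by branch ID, and ShrinkLeaves destroys meshes by that tag.
; A WateringCan-tagged overlap waters it once, plays the can's Niagara effect, then POSTs the issue key to a localhost completion endpoint.
; Thorn, weather, time-of-day and level-loading functions only print; the JSON header node is unwired.
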(event `SetWeather`
  (params (Weather_State :type String))
  (`KismetSystemLibrary.PrintString` Weather_State))

(event `Set_Time_Of_Day`
  (params (Progress_Ratio :type "Float (double-precision)"))
  (`KismetSystemLibrary.PrintString` "Hello" true true (struct :`G` 0.66 :`B` 1.0 :`A` 1.0) Progress_Ratio))

(event `self.Box.OnComponentBeginOverlap`
  (params (OverlappedComponent :type "PrimitiveComponent Object Reference") (OtherActor :type "Actor Object Reference") (OtherComp :type "PrimitiveComponent Object Reference") (OtherBodyIndex :type Integer) (bFromSweep :type Boolean) (SweepResult :type "HitResult Structure (by ref)"))
  (bind _returnvalue (`self.GetComponentByClass` OtherActor "/Script/Niagara.NiagaraComponent"))
  (if (`self.ActorHasTag` OtherActor "WateringCan")
    (if (not (`self.IsWatered`))
      (set `self.IsWatered` true)
      (`ActorComponent.Activate` _returnvalue false)
      (`KismetSystemLibrary.Delay` 2.0)
      (`self.Send_Complete_Task`)
      (`ActorComponent.Deactivate` _returnvalue))))

(event `Send_Complete_Task`
  (`HttpRequestProxyObject.CreateHttpRequestProxyObject` "http://localhost:5000/complete_task" "POST" (make `HttpHeader`) (`KismetStringLibrary.Concat_StrStr` "{\"issue_key\": \"" (`self.JiraIssueKey`) "\"}")))

(fn `Add_Thorns`
  (params (Target_Branch_ID :type String) (Epic_ID :type String))
  (`KismetSystemLibrary.PrintString` "🌵 Blocker detected!"))

(fn `Grow_Leaves`
  (params (Target_Branch_ID :type String) (Color_R :type "Float (double-precision)") (Color_G :type "Float (double-precision)") (Color_B :type "Float (double-precision)") (EpicID :type String) (Growth_Modifier :type "Float (double-precision)"))
  (bind _returnvalue (`AddComponent|NODE_AddStaticMeshComponent-0` :`RelativeTransform` (`KismetMathLibrary.MakeTransform` (0.0 0.0 100.0) (struct) (`KismetMathLibrary.Conv_DoubleToVector` Growth_Modifier))))
  (set `ActorComponent.ComponentTags` (`|MakeArray` (`KismetStringLibrary.Conv_StringToName` Target_Branch_ID)) _returnvalue)
  (`KismetSystemLibrary.PrintString` "MESH CREATED!")
  (`SceneComponent.K2_AttachToComponent` _returnvalue (`self.DefaultSceneRoot`) "None" "SnapToTarget" "SnapToTarget" "SnapToTarget" true)
  (`SceneComponent.K2_SetRelativeLocation` _returnvalue (0.0 0.0 100.0) false false))

(fn `Load_Generated_Level`
  (params (File_Path :type String))
  (`KismetSystemLibrary.PrintString` "Hello"))

(fn `Remove_Thorns`
  (params (Target_Branch_ID :type String))
  (`KismetSystemLibrary.PrintString` "✅ Blocker resolved!"))

(fn `Shrink_Leaves`
  (params (Target_Branch_ID :type String))
  (for _array_element (`self.GetComponentsByTag` "/Script/Engine.StaticMeshComponent" (`KismetStringLibrary.Conv_StringToName` Target_Branch_ID))
    (`ActorComponent.K2_DestroyComponent` _array_element)))

(fn `UserConstructionScript`)